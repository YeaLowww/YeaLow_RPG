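; Player inventory component that handles item pickup, money collection and the inventory, interact and health bar widgets.
; A forward sphere trace each tick drives the interact prompt; the interact input stacks items by DataTable stack size into resizable sword, shield and eatable slot arrays.
; Capsule overlaps collect money, the only value saved and loaded.
; IncreaseHealth writes to the character's damage component, DecreaseHealth to a local variable, with temporary N/M test keys.
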(event Custom|Collide%20With%20Item
  (params (OverlappedComponent :type Primitive%20Component%20Object%20Reference) (OtherActor :type Actor%20Object%20Reference) (OtherComp :type Primitive%20Component%20Object%20Reference) (OtherBodyIndex :type Integer) (bFromSweep :type Boolean) (SweepResult :type Hit%20Result%20Structure%20%28by%20ref%29))
  ;[1 1 1] Gaining Money
  (bind _asbp_money (Utilities|Casting|CastToBP_Money OtherActor))
  (bind _returnvalue (Utilities|GetDataTableRow "/Game/Inventory/Blueprints/DataTables/DT_Money.DT_Money" (.rowname (Variables|/Game/Inventory/Blueprints/Actors/BP_Money.BP_Money_C|GetDT_Money _asbp_money)))
    (:then
      (Variables|Money|SetMoneyGained (+ (.value _returnvalue) (Variables|Money|GetMoneyGained)))
      (Variables|/Game/Inventory/Blueprints/Widget/WBP_Inventory.WBP_Inventory_C|SetMoneyAmount (Variables|Widget|GetWBP_Inventory) (Variables|Money|GetMoneyGained))
      (Actor|DestroyActor _asbp_money))))

(event Input|EnhancedActionEvents|EnhancedInputActionIA_Interact
  (params (ActionValue :type Boolean) (ElapsedSeconds :type Float%20%28double-precision%29) (TriggeredSeconds :type Float%20%28double-precision%29) (InputAction :type Input%20Action%20Object%20Reference :default "/Game/ThirdPerson/Input/Actions/IA_Interact.IA_Interact"))
  ;[1 1 1] IA_Pickup
  (bind (_item _founditem _hitactor) (Inventory|TraceItemtoPickUp))
  (if _founditem
    (bind _success (Inventory|AddtoInventory _item))
    (if _success
      (Default|UpdateInventoryUI (Variables|Widget|GetWBP_Inventory) (Variables|Default|GetAllItems))
      (Actor|DestroyActor _hitactor))))

(event Input|EnhancedActionEvents|EnhancedInputActionIA_InventoryToggle
  (params (ActionValue :type Boolean) (ElapsedSeconds :type Float%20%28double-precision%29) (TriggeredSeconds :type Float%20%28double-precision%29) (InputAction :type Input%20Action%20Object%20Reference :default "/Game/Inventory/Blueprints/EnhancedInput/IA_InventoryToggle.IA_InventoryToggle"))
  (bind _returnvalue (Game|GetPlayerController 0))
  (bind _wbp_inventory (Variables|Widget|GetWBP_Inventory))
  ;[1 1 1] Opening Inventory
  (UserInterface|Viewport|AddtoViewport (Variables|Widget|GetWBP_Inventory) 0)
  (Variables|/Script/Engine.PlayerController|SetbShowMouseCursor _returnvalue true)
  (Input|SetInputModeUIOnly _returnvalue _wbp_inventory "DoNotLock" false)
  (Default|UpdateInventoryUI _wbp_inventory (Variables|Default|GetAllItems)))

(event EventBeginPlay
  (bind _allitems (Variables|Default|GetAllItems))
  ;[1 1 1] Begin Play
  (Class|BPIPersistance|RequestLoad(Message) (Game|GetGameInstance) self)
  (bind _returnvalue (UserInterface|CreateWidget "/Game/Inventory/Blueprints/Widget/WBP_Inventory.WBP_Inventory_C"))
  (Variables|Widget|SetWBP_Inventory _returnvalue)
  (bind _asbp_third_person_character (Utilities|Casting|CastToBP_ThirdPersonCharacter (Game|GetPlayerCharacter 0)))
  (bind _output_get (Variables|Private|SetAs%20BP%20Third%20Person%20Character _asbp_third_person_character))
  (Collision|BindEventtoOnComponentBeginOverlap (Variables|/Script/Engine.Character|GetCapsuleComponent _output_get) (EventDispatchers|CreateEvent :!event Custom|Collide%20With%20Item))
  (bind _returnvalue_2 (UserInterface|CreateWidget "/Game/Inventory/Blueprints/Widget/WBP_HealthBar.WBP_HealthBar_C"))
  (bind _output_get_2 (Variables|Widget|SetWBP_HealthBar _returnvalue_2))
  (Class|UserWidget|SetPositioninViewport _output_get_2 "(X=5.000000,Y=10.000000)" true)
  (UserInterface|Viewport|AddtoViewport _output_get_2 0)
  (bind _returnvalue_3 (UserInterface|CreateWidget "/Game/Inventory/Blueprints/Widget/WBP_Interact.WBP_Interact_C"))
  (Variables|Widget|SetWBP_Interact _returnvalue_3)
  (Utilities|Array|Resize (.swords _allitems) 4)
  (Utilities|Array|Resize (.shields _allitems) 6)
  (Utilities|Array|Resize (.eatables _allitems) 8)
  (Default|UpdateInventoryUI (Variables|Widget|GetWBP_Inventory) (Variables|Default|GetAllItems)))

(event EventTick
  (params (DeltaSeconds :type Float%20%28single-precision%29))
  (bind _wbp_interact (Variables|Widget|GetWBP_Interact))
  (bind _wbp_interact_2 (Variables|Widget|GetWBP_Interact))
  (bind _wbp_info (Variables|/Game/Inventory/Blueprints/Widget/WBP_Interact.WBP_Interact_C|GetWBP_Info _wbp_interact))
  ;[1 1 1] Event Tick
  (bind (_item _founditem) (Inventory|TraceItemtoPickUp))
  (Variables|/Game/Inventory/Blueprints/Widget/WBP_Info.WBP_Info_C|SetItem _wbp_info _item)
  (Default|UpdateItemInfo _wbp_info)
  (if _founditem
    (UserInterface|Viewport|AddtoViewport _wbp_interact_2 0)
    (else
      (Widget|RemovefromParent _wbp_interact_2))))

(event EventLoadData
  (params (SaveGameRef :type BP%20Save%20Game%20Object%20Reference))
  (Variables|Money|SetMoneyGained (Math|Float|Truncate (Variables|/Game/Save/BP_SaveGame.BP_SaveGame_C|GetCurency SaveGameRef))))

(event EventSaveData
  (params (SaveGameRef :type BP%20Save%20Game%20Object%20Reference))
  (Variables|/Game/Save/BP_SaveGame.BP_SaveGame_C|SetCurency SaveGameRef (Math|Conversions|ToFloat(Integer) (Variables|Money|GetMoneyGained))))

(event Input|KeyboardEvents|N
  (params (Key :type Key%20Structure :default "None"))
  ;[1 1 1] Temp
  (:Pressed
    (Health|IncreaseHealth 0.5)))

(event Input|KeyboardEvents|M
  (params (Key :type Key%20Structure :default "None"))
  ;[1 1 1] Temp
  (:Pressed
    (Health|DecreaseHealth 0.5)))

(fn IncreaseHealth
  (params (Health%20to%20Increase :type Float%20%28double-precision%29))
  (bind _asbp_third_person_character (Utilities|Casting|CastToBP_ThirdPersonCharacter (Game|GetPlayerCharacter 0)))
  (bind _health (Class|BPIDamageable|GetCurrentHealth(Message) _asbp_third_person_character))
  (bind _maxhealth (Class|BPIDamageable|GetMaxHealth(Message) _asbp_third_person_character))
  (if (>= (+ Health%20to%20Increase _health) _maxhealth)
    (Variables|/Game/DamageSystem/BPC_DamageSystem.BPC_DamageSystem_C|SetHealth (Variables|/Game/ThirdPerson/Blueprints/BP_ThirdPersonCharacter.BP_ThirdPersonCharacter_C|GetBPC_DamageSystem _asbp_third_person_character) _maxhealth)
    (else
      (Variables|/Game/DamageSystem/BPC_DamageSystem.BPC_DamageSystem_C|SetHealth (Variables|/Game/ThirdPerson/Blueprints/BP_ThirdPersonCharacter.BP_ThirdPersonCharacter_C|GetBPC_DamageSystem _asbp_third_person_character) (+ Health%20to%20Increase _health))))
  (Default|CallOnHealthChangedInv)
  (Default|UpdateHealth (Variables|Widget|GetWBP_HealthBar))
  (Default|UpdateHealth (Variables|/Game/Inventory/Blueprints/Widget/WBP_Inventory.WBP_Inventory_C|GetWBP_HealthBar (Variables|Widget|GetWBP_Inventory))))

(fn DecreaseHealth
  (params (Health%20to%20Decrease :type Float%20%28double-precision%29))
  (if (<= (- (Variables|HealthBar|GetHealth) Health%20to%20Decrease) 0.0)
    (Variables|HealthBar|SetHealth 0.0)
    (else
      (Variables|HealthBar|SetHealth (- (Variables|HealthBar|GetHealth) Health%20to%20Decrease))))
  (Default|UpdateHealth (Variables|Widget|GetWBP_HealthBar))
  (Default|UpdateHealth (Variables|/Game/Inventory/Blueprints/Widget/WBP_Inventory.WBP_Inventory_C|GetWBP_HealthBar (Variables|Widget|GetWBP_Inventory))))

(fn TraceItemtoPickUp
  (bind _returnvalue (Game|GetPlayerCharacter 0))
  (bind _returnvalue_2 (Transformation|GetActorLocation _returnvalue))
  (bind _returnvalue_3 (- _returnvalue_2 "0.000000,0.000000,60.000000"))
  (bind _outhit (Collision|SphereTraceByChannel _returnvalue_3 (+ _returnvalue_3 (* (Transformation|GetActorForwardVector _returnvalue) 1.5e+02)) 3e+01 "TraceTypeQuery1" false 0 "None"))
  (bind _asbp_items (Utilities|Casting|CastToBP_Items (.hitactor _outhit))
    (:then
      (Utilities|IsValid _asbp_items
        (:Is%20Valid
          (return (Variables|/Game/Inventory/Blueprints/Actors/BP_Items.BP_Items_C|GetItem _asbp_items) true (.hitactor _outhit)))))
    (:CastFailed
      (return "" false 0))))

(fn AddtoInventory
  (params (Item :type Struct%20Slot%20Structure))
  (bind _allitems (Variables|Default|GetAllItems))
  (bind (_itemid _quantity) (Utilities|Struct|BreakStruct_Slot Item))
  (bind (_itemid_2 _quantity_2) (Utilities|Struct|BreakStruct_Slot Item))
  (bind (_itemid_3 _quantity_3 _itemtype) (Utilities|Struct|BreakStruct_Slot Item))
  (bind (_itemid_4 _quantity_4 _itemtype_2) (Utilities|Struct|BreakStruct_Slot Item))
  (bind _itemid_5 (Utilities|Struct|BreakStruct_Slot Item))
  (bind _eatables (Utilities|Struct|BreakStruct_AllItem _allitems))
  (bind (_itemid_6 _quantity_5 _itemtype_3) (Utilities|Struct|BreakStruct_Slot Item))
  (bind _rowname (Utilities|Struct|BreakDataTableRowHandle _itemid_5))
  (switch Utilities|FlowControl|Switch|SwitchonE_ItemTypes (.ItemType (Utilities|Struct|BreakStruct_Slot Item))
    (:NewEnumerator0
      ;[1 1 1] Adding Similar swords to the same slot if stack space availabe
      (for (_array_element _array_index) (.Swords (Utilities|Struct|BreakStruct_AllItem (Variables|Default|GetAllItems)))
        (if (== (.RowName (Utilities|Struct|BreakDataTableRowHandle (.ItemID (Utilities|Struct|BreakStruct_Slot _array_element)))) (.RowName (Utilities|Struct|BreakDataTableRowHandle (.ItemID (Utilities|Struct|BreakStruct_Slot Item)))))
          (bind _returnvalue (Utilities|GetDataTableRow "/Game/Inventory/Blueprints/DataTables/DT_Items.DT_Items" (.RowName (Utilities|Struct|BreakDataTableRowHandle _itemid_2)))
            (:then
              (if (<= (+ (.Quantity (Utilities|Struct|BreakStruct_Slot _array_element)) _quantity_2) (.StackSize (Utilities|Struct|BreakStruct_Items _returnvalue)))
                (Utilities|Array|SetArrayElem (.Swords (Utilities|Struct|BreakStruct_AllItem (Variables|Default|GetAllItems))) _array_index (Utilities|Struct|MakeStruct_Slot _itemid_4 (+ (.Quantity (Utilities|Struct|BreakStruct_Slot _array_element)) _quantity_2) _itemtype_2))
                (return true))))))
      ;[1 1 1] Adding Different Sword Item to new slot or adding same item into a new slot if stack is full
      (for (_array_element_2 _array_index_2) (.Swords (Utilities|Struct|BreakStruct_AllItem (Variables|Default|GetAllItems)))
        (if (== (.Quantity (Utilities|Struct|BreakStruct_Slot _array_element_2)) 0)
          (Utilities|Array|SetArrayElem (.Swords (Utilities|Struct|BreakStruct_AllItem (Variables|Default|GetAllItems))) _array_index_2 Item)
          (return true)))
      (return false))
    (:NewEnumerator1
      ;[1 1 1] Adding Similar shields to the same slot if stack space availabe
      (for (_array_element_3 _array_index_3) (.Shields (Utilities|Struct|BreakStruct_AllItem (Variables|Default|GetAllItems)))
        (if (== (.rowname (.ItemID (Utilities|Struct|BreakStruct_Slot _array_element_3))) _rowname)
          (bind _returnvalue_2 (Utilities|GetDataTableRow "/Game/Inventory/Blueprints/DataTables/DT_Items.DT_Items" _rowname)
            (:then
              (if (<= (+ (.Quantity (Utilities|Struct|BreakStruct_Slot _array_element_3)) (.Quantity (Utilities|Struct|BreakStruct_Slot Item))) (.StackSize (Utilities|Struct|BreakStruct_Items _returnvalue_2)))
                (Utilities|Array|SetArrayElem (.Shields (Utilities|Struct|BreakStruct_AllItem (Variables|Default|GetAllItems))) _array_index_3 (Utilities|Struct|MakeStruct_Slot _itemid_6 (+ (.Quantity (Utilities|Struct|BreakStruct_Slot _array_element_3)) (.Quantity (Utilities|Struct|BreakStruct_Slot Item))) _itemtype_3))
                (return true))))))
      ;[1 1 1] Adding Different shield Item to new slot or adding same item into a new slot if stack is full
      (for (_array_element_4 _array_index_4) (.Shields (Utilities|Struct|BreakStruct_AllItem (Variables|Default|GetAllItems)))
        (if (== (.Quantity (Utilities|Struct|BreakStruct_Slot _array_element_4)) 0)
          (Utilities|Array|SetArrayElem (.Shields (Utilities|Struct|BreakStruct_AllItem (Variables|Default|GetAllItems))) _array_index_4 Item)
          (return true)))
      (return false))
    (:NewEnumerator2
      ;[1 1 1] Adding Similar eatables to the same slot if stack space availabe
      (for (_array_element_5 _array_index_5) (.eatables (Variables|Default|GetAllItems))
        (if (== (.RowName (Utilities|Struct|BreakDataTableRowHandle (.ItemID (Utilities|Struct|BreakStruct_Slot _array_element_5)))) (.rowname (.ItemID (Utilities|Struct|BreakStruct_Slot Item))))
          (bind _returnvalue_3 (Utilities|GetDataTableRow "/Game/Inventory/Blueprints/DataTables/DT_Items.DT_Items" (.rowname _itemid))
            (:then
              (if (<= (+ _quantity (.Quantity (Utilities|Struct|BreakStruct_Slot _array_element_5))) (.StackSize (Utilities|Struct|BreakStruct_Items _returnvalue_3)))
                (Utilities|Array|SetArrayElem (.Eatables (Utilities|Struct|BreakStruct_AllItem (Variables|Default|GetAllItems))) _array_index_5 (Utilities|Struct|MakeStruct_Slot _itemid_3 (+ _quantity (.Quantity (Utilities|Struct|BreakStruct_Slot _array_element_5))) _itemtype))
                (return true))))))
      ;[1 1 1] Adding Different eatable Item to new slot or adding same item into a new slot if stack is full
      (for (_array_element_6 _array_index_6) _eatables
        (if (== (.Quantity (Utilities|Struct|BreakStruct_Slot _array_element_6)) 0)
          (Utilities|Array|SetArrayElem _eatables _array_index_6 Item)
          (return true)))
      (return false))))

(fn UpgradeInventory
  (params (SwordsAmount :type Integer) (ShieldsAmount :type Integer) (EatablesAmount :type Integer))
  (bind _allitems (Variables|Default|GetAllItems))
  (bind (_swords _shields _eatables) (Utilities|Struct|BreakStruct_AllItem _allitems))
  (Utilities|Array|Resize _swords (+ SwordsAmount (Utilities|Array|Length _swords)))
  (Utilities|Array|Resize _shields (+ ShieldsAmount (Utilities|Array|Length _shields)))
  (Utilities|Array|Resize _eatables (+ EatablesAmount (Utilities|Array|Length _eatables)))
  (Default|UpdateInventoryUI (Variables|Widget|GetWBP_Inventory) (Variables|Default|GetAllItems)))