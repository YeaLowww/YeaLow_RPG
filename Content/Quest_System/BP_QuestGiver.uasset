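; Quest giver actor that plays dialogue and then shows its list of quests.
; A trigger radius toggles the interact prompt for the player character, and Tick turns that prompt toward the camera.
; Each Interact advances the Dialogue array in a dialogue widget; passing the end opens the quests widget, filled from Quests.
; Interacting again or calling CloseWidget removes the quests widget and restores game-only input.
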(event OnComponentBeginOverlap(TriggerRadius)
  (params (OverlappedComponent :type Primitive%20Component%20Object%20Reference) (OtherActor :type Actor%20Object%20Reference) (OtherComp :type Primitive%20Component%20Object%20Reference) (OtherBodyIndex :type Integer) (bFromSweep :type Boolean) (SweepResult :type Hit%20Result%20Structure%20%28by%20ref%29))
  ;[0.05127 0.05127 0.05127] Visibility text Assassination
  (Utilities|Casting|CastToBP_ThirdPersonCharacter OtherActor)
  (Rendering|SetVisibility (Variables|Default|GetInteract%20Widget) true false))

(event OnComponentEndOverlap(TriggerRadius)
  (params (OverlappedComponent :type Primitive%20Component%20Object%20Reference) (OtherActor :type Actor%20Object%20Reference) (OtherComp :type Primitive%20Component%20Object%20Reference) (OtherBodyIndex :type Integer))
  ;[0.05127 0.05127 0.05127] Visibility text Assassination
  (Utilities|Casting|CastToBP_ThirdPersonCharacter OtherActor)
  (Rendering|SetVisibility (Variables|Default|GetInteract%20Widget) false false))

(event Custom|Close%20Widget
  (bind _returnvalue (Game|GetPlayerController 0))
  (Widget|RemovefromParent (Variables|Default|GetQuests%20Widget))
  (Variables|Default|SetQuests%20Widget 0)
  (Variables|/Script/Engine.PlayerController|SetbShowMouseCursor _returnvalue false)
  (Input|SetInputModeGameOnly _returnvalue false)
  (Variables|Default|SetWidgetActive false))

(event Custom|Open%20Quests%20Widget
  (bind _returnvalue (UserInterface|CreateWidget "/Game/Quest_System/WB_QuestGiver.WB_QuestGiver_C"))
  (bind _output_get (Variables|Default|SetQuests%20Widget _returnvalue))
  (UserInterface|Viewport|AddtoViewport _output_get 0)
  (Variables|Default|SetWidgetActive true)
  (Variables|/Game/Quest_System/WB_QuestGiver.WB_QuestGiver_C|SetQuest%20Giver%20BP (Variables|Default|GetQuests%20Widget) self)
  (for _array_element (Variables|Default|GetQuests)
    (Default|AddQuest (Variables|Default|GetQuests%20Widget) _array_element)))

(event EventInteract
  (bind _returnvalue (Game|GetPlayerController 0))
  (bind _returnvalue_2 (Game|GetPlayerController 0))
  (if (not (Variables|Default|GetWidgetActive))
    (if (not (Variables|Default|GetdialogueOpened?))
      (bind _returnvalue_3 (UserInterface|CreateWidget "/Game/Quest_System/WB_QuestGiverDialogue.WB_QuestGiverDialogue_C"))
      (bind _output_get (Variables|Default|SetDialogue%20Widget _returnvalue_3))
      (UserInterface|Viewport|AddtoViewport _output_get 0)
      (Variables|Default|SetdialogueOpened? true)
      (Rendering|Components|TextRender|SetText (Variables|/Game/Quest_System/WB_QuestGiverDialogue.WB_QuestGiverDialogue_C|GetDialogueText (Variables|Default|GetDialogue%20Widget)) (Utilities|Text|ToText(String) (Utilities|Array|Get(acopy) (Variables|Default|Getdialogue) (Variables|Default|GetdialogueIndex))))
      (Math|Integer|IncrementInt (Variables|Default|GetdialogueIndex)
        (:%20%20
          (Variables|/Script/Engine.PlayerController|SetbShowMouseCursor _returnvalue_2 true)
          (Input|SetInputModeGameandUI _returnvalue_2 (Variables|Default|GetQuests%20Widget) "DoNotLock" true false)))
      (else
        (Rendering|Components|TextRender|SetText (Variables|/Game/Quest_System/WB_QuestGiverDialogue.WB_QuestGiverDialogue_C|GetDialogueText (Variables|Default|GetDialogue%20Widget)) (Utilities|Text|ToText(String) (Utilities|Array|Get(acopy) (Variables|Default|Getdialogue) (Variables|Default|GetdialogueIndex))))
        (Math|Integer|IncrementInt (Variables|Default|GetdialogueIndex)
          (:%20%20
            (if (> (Variables|Default|GetdialogueIndex) (Utilities|Array|Length (Variables|Default|Getdialogue)))
              (Widget|RemovefromParent (Variables|Default|GetDialogue%20Widget))
              (Variables|Default|SetDialogue%20Widget 0)
              (Variables|Default|SetdialogueIndex 0)
              (Variables|Default|SetdialogueOpened? false)
              (CallFunction|OpenQuestsWidget))))))
    (else
      (Widget|RemovefromParent (Variables|Default|GetQuests%20Widget))
      (Variables|Default|SetQuests%20Widget 0)
      (Variables|/Script/Engine.PlayerController|SetbShowMouseCursor _returnvalue false)
      (Input|SetInputModeGameOnly _returnvalue false)
      (Variables|Default|SetWidgetActive false))))

(event Collision|EventActorBeginOverlap
  (params (OtherActor :type Actor%20Object%20Reference)))

(event EventTick
  (params (DeltaSeconds :type Float%20%28single-precision%29))
  (Transformation|SetWorldRotation (Variables|Default|GetInteract%20Widget) (Math|Rotator|FindLookatRotation (Transformation|GetWorldLocation (Variables|Default|GetInteract%20Widget)) (Transformation|GetWorldLocation (Variables|/Script/Engine.PlayerCameraManager|GetTransformComponent (Game|GetPlayerCameraManager 0)))) false false))

(fn ConstructionScript)