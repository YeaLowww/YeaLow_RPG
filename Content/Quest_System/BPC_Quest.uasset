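; Quest component that tracks a single active quest and its enemy-elimination and chest-opening objectives.
; It creates the quest HUD widget on BeginPlay, hidden at first, and fills it with the quest name and objectives.
; Kill and chest events update matching objective structs by reference, using a shared working array for remaining enemies.
; Each completion updates the HUD and a counter, which clears the quest and plays the completion animation when all are done.
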(event Custom|Set%20Active%20Quest%20Text
  (Rendering|Components|TextRender|SetText (Variables|/Game/Quest_System/WB_QuestHUD.WB_QuestHUD_C|GetActiveQuestText (Variables|Default|GetQuestHUD%20Widget)) (Utilities|Text|ToText(String) (.Name (Utilities|Struct|BreakS_Quest (Variables|Default|GetactiveQuest)))))
  (Default|ShowQuestPanel (Variables|Default|GetQuestHUD%20Widget)))

(event Custom|Set%20Objectives
  (Default|FillObjectives (Variables|Default|GetQuestHUD%20Widget) (.objectives (Variables|Default|GetactiveQuest))))

(event Custom|Open%20Chest
  (params (Chest :type Actor%20Object%20Reference))
  (for _array_element (.objectives (Variables|Default|GetactiveQuest))
    (if (and (.isChestObjective (Utilities|Struct|BreakS_Quest_Objective _array_element)) (== Chest (.ChesttoOpen (Utilities|Struct|BreakS_Quest_Objective _array_element))))
      (|SetBy-RefVar _array_element (Utilities|Struct|MakeS_Quest_Objective (.NameAim (Utilities|Struct|BreakS_Quest_Objective _array_element)) true (.ActorstoEliminate (Utilities|Struct|BreakS_Quest_Objective _array_element)) 0 (.isEliminateEnemyObjective (Utilities|Struct|BreakS_Quest_Objective _array_element)) (.isChestObjective (Utilities|Struct|BreakS_Quest_Objective _array_element))))
      (Default|CompletedObjective (Variables|Default|GetQuestHUD%20Widget) _array_element)
      (CallFunction|ObjectiveCompleted)
      (Development|PrintString "Competed"))))

(event Custom|Eliminate%20Enemy
  (params (Enemy%20Eliminated :type Actor%20Object%20Reference))
  (for _array_element (.objectives (Variables|Default|GetactiveQuest))
    (if (and (not (.Completed (Utilities|Struct|BreakS_Quest_Objective _array_element))) (.isEliminateEnemyObjective (Utilities|Struct|BreakS_Quest_Objective _array_element)))
      (if (!= (Utilities|Array|Length (Variables|Default|GetEnemy%20Actors%20Array)) 0)
        _
        (else
          (bind _output_get (Variables|Default|SetEnemy%20Actors%20Array (.ActorstoEliminate (Utilities|Struct|BreakS_Quest_Objective _array_element))))))
      (Utilities|Array|RemoveItem _output_get Enemy%20Eliminated)
      (|SetBy-RefVar _array_element (Utilities|Struct|MakeS_Quest_Objective (.NameAim (Utilities|Struct|BreakS_Quest_Objective _array_element)) false (Variables|Default|GetEnemy%20Actors%20Array) (.ChesttoOpen (Utilities|Struct|BreakS_Quest_Objective _array_element)) (.isEliminateEnemyObjective (Utilities|Struct|BreakS_Quest_Objective _array_element)) (.isChestObjective (Utilities|Struct|BreakS_Quest_Objective _array_element))))
      (Development|PrintString (Utilities|String|ToString(Integer) (Utilities|Array|Length (Variables|Default|GetEnemy%20Actors%20Array))))
      (if (== (Utilities|Array|Length (Variables|Default|GetEnemy%20Actors%20Array)) 0)
        (|SetBy-RefVar _array_element (Utilities|Struct|MakeS_Quest_Objective (.NameAim (Utilities|Struct|BreakS_Quest_Objective _array_element)) true 0 (.ChesttoOpen (Utilities|Struct|BreakS_Quest_Objective _array_element)) (.isEliminateEnemyObjective (Utilities|Struct|BreakS_Quest_Objective _array_element)) (.isChestObjective (Utilities|Struct|BreakS_Quest_Objective _array_element))))
        (Default|CompletedObjective (Variables|Default|GetQuestHUD%20Widget) _array_element)
        (CallFunction|ObjectiveCompleted)
        (Development|PrintString "Competed")))))

(event Custom|Objective%20Completed
  (Math|Integer|IncrementInt (Variables|Default|GetObjectives%20Completed)
    (:%20%20
      (if (>= (Variables|Default|GetObjectives%20Completed) (Utilities|Array|Length (.objectives (Variables|Default|GetactiveQuest))))
        (Variables|Default|SetactiveQuest "")
        (Variables|Default|SetObjectives%20Completed 0)
        (Default|PlayQuestCompletedAnim (Variables|Default|GetQuestHUD%20Widget))))))

(event EventBeginPlay
  (bind _returnvalue (UserInterface|CreateWidget "/Game/Quest_System/WB_QuestHUD.WB_QuestHUD_C"))
  (bind _output_get (Variables|Default|SetQuestHUD%20Widget _returnvalue))
  (UserInterface|Viewport|AddtoViewport _output_get 0)
  (Default|HideQuestPanel (Variables|Default|GetQuestHUD%20Widget)))