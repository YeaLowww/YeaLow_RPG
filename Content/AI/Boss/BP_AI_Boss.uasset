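; BP_AI_Boss is the boss AI character, with health tracking and support for being the victim of a stealth back assassination.
; Every Tick it casts its controller to BP_AIController_Boss and copies current health from BPCPlayerStats into it; the MaxHealth copy is unconnected.
; StealthBackAssassin plays the victim's paired knife montage and returns the AssassinREF world location and the boss's rotation.
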(event EventBeginPlay
  (|CallParentFunction) ; This node is disabled and will not be called.\nDrag off pins to build functionality.
)

(event Collision|EventActorBeginOverlap
  (params (OtherActor :type Actor%20Object%20Reference))
  (|CallParentFunction OtherActor) ; This node is disabled and will not be called.\nDrag off pins to build functionality.
)

(event EventTick
  (params (DeltaSeconds :type Float%20%28single-precision%29))
  (|CallParentFunction DeltaSeconds)
  (bind _asbp_aicontroller_boss (Utilities|Casting|CastToBP_AIController_Boss (AI|GetAIController self)))
  (Variables|/Game/AI/Boss/BP_AIController_Boss.BP_AIController_Boss_C|SetHealth _asbp_aicontroller_boss (Variables|/Game/Blueprints/BPC_PlayerStats.BPC_PlayerStats_C|GetCurrent%20Health (Variables|Default|GetBPC_PlayerStats))))

(fn ConstructionScript
  (|CallParentFunction))

(fn StealthBackAssassin
  (Animation|PlayAnimMontage "/Game/Characters/RPG_Character/Animation/Assassination/Paired_Knife_Stealth_KidneyAndNeck_Vic_Montage.Paired_Knife_Stealth_KidneyAndNeck_Vic_Montage" 1.0 "None")
  (return (Transformation|GetWorldLocation (Variables|Default|GetAssassin%20REF)) (Transformation|GetActorRotation)))