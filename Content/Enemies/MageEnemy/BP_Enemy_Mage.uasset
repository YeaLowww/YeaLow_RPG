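; BP_Enemy_Mage is a mage enemy with three attacks, a teleport and a heal over time.
; Attacks pass montage and damage info to BPCAttacks, while overrides supply movement speeds and ideal combat ranges.
; Teleport is a disguised fast flight: the mesh hides behind particles, pawn collision is ignored and AIMoveTo travels to the destination.
; Healing spawns an AOE during a montage, restoring the mage's health on overlap events.
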(event Custom|Teleport
  (params (Location :type Vector))
  (bind _charactermovement (Variables|Character|GetCharacterMovement))
  ;[1 1 1] Teleport
  (if (not (Variables|Default|GetisTeleporting))
    (Variables|Default|SetisTeleporting true)
    (Pawn|Components|CharacterMovement|SetMovementMode _charactermovement "MOVE_Flying" 0)
    (Variables|/Script/Engine.CharacterMovementComponent|SetMaxFlySpeed _charactermovement 5e+03)
    (Variables|/Script/Engine.CharacterMovementComponent|SetMaxAcceleration _charactermovement 99999.0)
    (Rendering|SetVisibility (Variables|Character|GetMesh) false true)
    (Collision|SetCollisionResponsetoChannel (Variables|Default|GetCapsuleComponent) "ECC_Pawn" "ECR_Ignore")
    (bind _returnvalue (Effects|SpawnEmitterAttached "/Game/StarterContent/Particles/P_Explosion.P_Explosion" (Variables|Character|GetMesh) "Spine1"))
    (Variables|Default|SetTeleportBodyEffect _returnvalue)
    (bind _returnvalue_2 (Effects|SpawnEmitterAttached "/Game/InfinityBladeEffects/Effects/FX_Mobile/Fire/combat/P_FireBall_Base_Trail.P_FireBall_Base_Trail" (Variables|Character|GetMesh) "Spine1"))
    (Variables|Default|SetTeleport%20Trail%20Effect _returnvalue_2)
    (Animation|StopAnimMontage 0)
    (AI|AIMoveTo self Location 0 15.0 false
      (:OnSuccess
        _)
      (:OnFail
        _))
    (CallFunction|TeleportEnd)
    (else
      (Utilities|FlowControl|DelayUntilNextTick)
      (Default|CallOnTeleportEnd))))

(event Custom|Teleport%20End
  (bind _charactermovement (Variables|Character|GetCharacterMovement))
  ;[1 1 1] Teleport
  (Components|Movement|StopMovementImmediately _charactermovement)
  (Pawn|Components|CharacterMovement|SetMovementMode _charactermovement "MOVE_Walking" 0)
  (Variables|/Script/Engine.CharacterMovementComponent|SetMaxAcceleration _charactermovement 1.5e+03)
  (Rendering|SetVisibility (Variables|Character|GetMesh) true true)
  (Collision|SetCollisionResponsetoChannel (Variables|Default|GetCapsuleComponent) "ECC_Pawn" "ECR_Block")
  (Default|CallOnTeleportEnd)
  (Utilities|FlowControl|Delay 0.5)
  (Variables|Default|SetisTeleporting false)
  (Utilities|FlowControl|Sequence
    (:then_0
      (bind _teleportbodyeffect (Variables|Default|GetTeleportBodyEffect)
        (:then
          (Components|DestroyComponent _teleportbodyeffect))
        (:else)))
    (:then_1
      (bind _teleport_trail_effect (Variables|Default|GetTeleport%20Trail%20Effect)
        (:then
          (Components|DestroyComponent _teleport_trail_effect))
        (:else)))))

(event Custom|HealOverTime
  ;[1 1 1] Heal
  (Animation|Montage|PlayMontage (Variables|Character|GetMesh) "/Game/MixamoMage/Standing_2H_Magic_Heal_Montage.Standing_2H_Magic_Heal_Montage"
    (:then
      (bind _returnvalue (Game|SpawnActorfromClass "/Game/AOE/BP_AOE_Heal.BP_AOE_Heal_C" (Math|Transform|MakeTransform (Transformation|GetSocketLocation (Variables|Character|GetMesh) "Spine1") "0, 0, 0" "1.000000,1.000000,1.000000") "Undefined" "MultiplyWithRoot" 0 1.0 1e+01 false false true 0))
      (bind _output_get (Variables|Default|SetHeal%20AOE _returnvalue))
      (EventDispatchers|AssignOnAOEOverlapActor _output_get (delegate Custom|OnHealTick)))
    (:OnCompleted
      (CallFunction|HealOverTimeEnded :!label _label))
    (:OnInterrupted
      (goto _label))))

(event Custom|HealOverTimeEnded
  ;[1 1 1] Heal
  (Default|CallOnHealOverTimeEnded)
  (bind _heal_aoe (Variables|Default|GetHeal%20AOE)
    (:then
      (Actor|DestroyActor _heal_aoe))
    (:else)))

(event Custom|OnHealTick
  (params (Actor :type Actor%20Object%20Reference))
  ;[1 1 1] Heal
  (if (== Actor self)
    (CallFunction|Heal (* (Variables|/Game/DamageSystem/BPC_DamageSystem.BPC_DamageSystem_C|GetMaxHealth (Variables|Default|GetBPC_DamageSystem)) 0.1))))

(event Custom|CastAttack
  (params (AttackTarget :type Actor%20Object%20Reference))
  ;[1 1 1] Attacks
  (Default|CastMageAttack (Variables|Default|GetBPC_Attacks) (Utilities|Struct|MakeS_AttackInfo AttackTarget "/Game/Animation/AnimFromMixamo/Montages/Standing_Cast_Magic_Attack_Montage.Standing_Cast_Magic_Attack_Montage" (Utilities|Struct|MakeS_DamageInfo 0.0 "NewEnumerator2"))))

(event Custom|BasicAttack
  (params (AttackTarget :type Actor%20Object%20Reference))
  ;[1 1 1] Attacks
  (Default|BasicMageSpell (Variables|Default|GetBPC_Attacks) (Utilities|Struct|MakeS_AttackInfo AttackTarget "/Game/MixamoMage/Fireball_Montage.Fireball_Montage" (Utilities|Struct|MakeS_DamageInfo 0.0 "NewEnumerator2"))))

(event Custom|GroundSmashAttack
  (params (AttackTarget :type Actor%20Object%20Reference))
  ;[1 1 1] Attacks
  (Default|GroundSmash (Variables|Default|GetBPC_Attacks) (Utilities|Struct|MakeS_AttackInfo AttackTarget "/Game/Animation/AnimFromMixamo/Montages/MageGroundSmash_Montage.MageGroundSmash_Montage" (Utilities|Struct|MakeS_DamageInfo 0.0 "NewEnumerator3")) 3e+02))

(fn ConstructionScript
  (|CallParentFunction))

(fn SetMovementSpeed
  (params (Speed :type E_MovementSpeed%20Enum :default "NewEnumerator0"))
  (return (Utilities|Select :Index Speed :NewEnumerator0 0.0 :NewEnumerator1 1.5e+02 :NewEnumerator2 2e+02 :NewEnumerator3 4e+02)))

(fn GetIdealRange
  (return 5e+02 7e+02))