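; Ranged enemy Blueprint that fights with a rifle, extending a parent enemy's begin play and attack logic.
; On BeginPlay it spawns a rifle, attaches it to the right-hand socket and signals that the weapon is equipped.
; Attacks play a fire montage whose notify has BPCAttacks fire blockable bullets from weapon to target, ending the attack on completion or interruption.
; SetMovementSpeed maps speed states to walk speeds.
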(event EventEquipWeapon
  (bind _returnvalue (Game|SpawnActorfromClass "/Game/Weapons/BP_Weapon_Rifle.BP_Weapon_Rifle_C" (Math|Transform|MakeTransform "0, 0, 0") "Undefined" "MultiplyWithRoot" 0 0))
  (bind _output_get (Variables|Default|SetWeaponActor _returnvalue))
  (Transformation|AttachComponentToComponent _output_get (Variables|Character|GetMesh) "hand_rSocket Rifle" "SnapToTarget" "SnapToTarget" "SnapToTarget" true)
  (Variables|Default|SetisWieldingWeapon true)
  (Default|CallOnWeaponEquipped))

(event EventBeginPlay
  (|CallParentFunction)
  (CallFunction|EquipWeapon))

(event EventAttack
  (params (AttackTarget :type Actor%20Object%20Reference))
  (|CallParentFunction AttackTarget)
  (bind _notifyname (Animation|Montage|PlayMontage (Variables|Character|GetMesh) "/Game/Animation/Rifle/rifle-fire_Montage.rifle-fire_Montage")
    (:OnCompleted
      (CallFunction|AttackEnd AttackTarget :!label _label))
    (:OnInterrupted
      (goto _label))
    (:OnNotifyBegin
      (switch name _notifyname
        (:Fire
          (Default|FireBullets (Variables|Default|GetBPC_Attacks) (Transformation|GetActorLocation (Variables|Default|GetWeaponActor)) (Transformation|GetActorLocation AttackTarget) (Utilities|Struct|MakeS_DamageInfo 0.0 "NewEnumerator2" "NewEnumerator0" false true)))))))

(fn ConstructionScript
  (|CallParentFunction))

(fn SetMovementSpeed
  (params (Speed :type E_MovementSpeed%20Enum :default "NewEnumerator0"))
  (bind _output_get (Variables|/Script/Engine.CharacterMovementComponent|SetMaxWalkSpeed (Variables|Character|GetCharacterMovement) (Utilities|Select :Index Speed :NewEnumerator0 0.0 :NewEnumerator1 2e+02 :NewEnumerator2 3e+02 :NewEnumerator3 5e+02)))
  (return _output_get))