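; Sword-wielding melee enemy Blueprint with short-range, long-range jump, ground smash and spinning attacks, plus montage-driven sword equip and unequip.
; Standard attacks pass montage and damage info to BPCAttacks.
; The uninterruptible spin attack uses montage notifies to start a timeline-driven mesh yaw spin while repeatedly chasing the target, and to spawn an AOE actor that damages only that target.
; Notifies also spawn or destroy the hand-socketed sword.
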(event Custom|StopSpinning
  ;[1 1 1] Attack Helpers For Spinner
  (Audio|Components|Audio|Stop (Variables|Default|GetSpinMesh%20Timeline))
  (Transformation|SetRelativeRotation (Variables|Character|GetMesh) (Variables|Default|GetMeshRotationBeforeSpin) false false))

(event Custom|AOESlash
  (params (AttackTarget :type Actor%20Object%20Reference))
  ;[1 1 1] Attack Helpers For Spinner
  (bind _returnvalue (Game|SpawnActorfromClass "/Game/AOE/BP_AOE_Base.BP_AOE_Base_C" (Math|Transform|MakeTransform (Transformation|GetActorLocation) "0, 0, 0" "1.000000,1.000000,1.000000") "Undefined" "MultiplyWithRoot" 0 false true false self))
  (Variables|/Game/AOE/BP_AOE_Base.BP_AOE_Base_C|SetRadius _returnvalue 3e+02)
  (EventDispatchers|AssignOnAOEOverlapActor _returnvalue (delegate Custom|AOEDamageActor))
  (Default|Trigger _returnvalue))

(event Custom|AOEDamageActor
  (params (Actor :type Actor%20Object%20Reference))
  ;[1 1 1] Attack Helpers For Spinner
  (if (== Actor (stale Custom|AOESlash AttackTarget))
    (Class|BPIDamageable|TakeDamage(Message) Actor (Utilities|Struct|MakeS_DamageInfo 0.0 "NewEnumerator1" "NewEnumerator1" false true) self)))

(event Custom|Spinning%20Attack
  (params (AttackTarget :type Actor%20Object%20Reference))
  ;[1 1 1] Attack
  (|CallParentFunction AttackTarget)
  (bind _notifyname (Animation|Montage|PlayMontage (Variables|Character|GetMesh) "/Game/Animation/AnimFromMixamo/Montages/SwordSpinnerAttack_UE_Montage.SwordSpinnerAttack_UE_Montage")
    (:then
      (Variables|/Game/DamageSystem/BPC_DamageSystem.BPC_DamageSystem_C|SetIsInterruptible (Variables|Default|GetBPC_DamageSystem) false))
    (:OnCompleted
      (CallFunction|AttackEnd AttackTarget :!label _label)
      (Variables|/Game/DamageSystem/BPC_DamageSystem.BPC_DamageSystem_C|SetIsInterruptible (Variables|Default|GetBPC_DamageSystem) true)
      (CallFunction|StopSpinning))
    (:OnInterrupted
      (goto _label))
    (:OnNotifyBegin
      (switch name _notifyname
        (:Spin
          (CallFunction|SpinMesh)
          (CallFunction|ChaseAttackTarget AttackTarget))
        (:AOESlash
          (CallFunction|AOESlash AttackTarget))))))

(event Custom|LongRangeAttack
  (params (AttackTarget :type Actor%20Object%20Reference))
  ;[1 1 1] Attack
  (Default|LongRangeMeleeAttack (Variables|Default|GetBPC_Attacks) (Utilities|Struct|MakeS_AttackInfo AttackTarget "/Game/Animation/AnimFromMixamo/Montages/SwordJumpAttack_UE_Montage.SwordJumpAttack_UE_Montage" (Utilities|Struct|MakeS_DamageInfo 0.0 "NewEnumerator1" "NewEnumerator0" false true true))))

(event Custom|ShortRangeAttack
  (params (AttackTarget :type Actor%20Object%20Reference))
  ;[1 1 1] Attack
  (Default|PrimaryMeleeAttack (Variables|Default|GetBPC_Attacks) (Utilities|Struct|MakeS_AttackInfo AttackTarget "/Game/Animation/Melee/sword-slash_Montage.sword-slash_Montage" (Utilities|Struct|MakeS_DamageInfo 0.0 "NewEnumerator1" "NewEnumerator0" false true true)) 2e+01 2e+02))

(event Custom|GroundSmashAttack
  (params (AttackTarget :type Actor%20Object%20Reference))
  ;[1 1 1] Attack
  (Default|GroundSmash (Variables|Default|GetBPC_Attacks) (Utilities|Struct|MakeS_AttackInfo AttackTarget "/Game/Animation/AnimFromMixamo/Montages/MeleeGroundSmash.MeleeGroundSmash" (Utilities|Struct|MakeS_DamageInfo 0.0 "NewEnumerator3")) 3e+02))

(event Custom|Spin%20Mesh
  ;[1 1 1] Attack Helpers For Spinner
  (Variables|Default|SetMeshRotationBeforeSpin (Variables|/Script/Engine.SceneComponent|GetRelativeRotation (Variables|Character|GetMesh)))
  (bind _zrotationalpha (Timeline|SpinMesh%20Timeline PlayFromStart)
    (:Update
      (Transformation|SetRelativeRotation (Variables|Character|GetMesh) (Math|Rotator|MakeRotator (.roll (Variables|Default|GetMeshRotationBeforeSpin)) (.pitch (Variables|Default|GetMeshRotationBeforeSpin)) (Math|Float|Lerp (.yaw (Variables|Default|GetMeshRotationBeforeSpin)) (+ (.yaw (Variables|Default|GetMeshRotationBeforeSpin)) 4.32e+03) _zrotationalpha)) false false))))

(event Custom|ChaseAttackTarget
  (params (AttackTarget :type Actor%20Object%20Reference))
  ;[1 1 1] Attack Helpers For Spinner
  (AI|AIMoveTo self "0, 0, 0" AttackTarget 2e+02 false
    (:OnSuccess
      (Utilities|FlowControl|Delay 0.1)
      (if (Variables|Default|GetAttacking)
        (CallFunction|ChaseAttackTarget AttackTarget)))))

(event EventBeginPlay
  (|CallParentFunction))

(event EventEquipWeapon
  ;[1 1 1] Equip weapon
  (bind _notifyname (Animation|Montage|PlayMontage (Variables|Character|GetMesh) "/Game/Animation/SheathSword/UnSheathing_Sword_Montage.UnSheathing_Sword_Montage")
    (:OnCompleted
      (Default|CallOnWeaponEquipped))
    (:OnNotifyBegin
      (switch name _notifyname
        (:Open%20Sword
          (bind _returnvalue (Game|SpawnActorfromClass "/Game/Weapons/BP_Weapon_Sword.BP_Weapon_Sword_C" (Transformation|GetActorTransform) "Undefined" "MultiplyWithRoot" 0 0))
          (Variables|Default|SetWeaponActor _returnvalue)
          (Transformation|AttachComponentToComponent _returnvalue (Variables|Character|GetMesh) "hand_rSocket Sword" "SnapToTarget" "SnapToTarget" "SnapToTarget" true)
          (Variables|Default|SetisWieldingWeapon true))))))

(event EventUnEquipWeapon
  ;[1 1 1] Equip weapon
  (bind _notifyname (Animation|Montage|PlayMontage (Variables|Character|GetMesh) "/Game/Animation/SheathSword/Sheathing_Sword_Montage.Sheathing_Sword_Montage")
    (:OnCompleted
      (Default|CallOnWeaponUnEquipped))
    (:OnNotifyBegin
      (switch name _notifyname
        (:Drop%20Sword
          (Actor|DestroyActor (Variables|Default|GetWeaponActor))
          (Variables|Default|SetisWieldingWeapon false))))))

(fn ConstructionScript
  (|CallParentFunction)
  (Variables|Default|SetMeshRotationBeforeSpin (Variables|/Script/Engine.SceneComponent|GetRelativeRotation (Variables|Character|GetMesh))))

(fn IsDead
  (return (Variables|/Game/DamageSystem/BPC_DamageSystem.BPC_DamageSystem_C|GetIsDead (Variables|Default|GetBPC_DamageSystem))))

(fn GetIdealRange
  (return 2e+02 4e+02))

(fn CalculateFutureActorLocation
  (params (Actor :type Actor%20Object%20Reference) (Time :type Float%20%28double-precision%29))
  ;[1 1 1] location = velocity * time +currLocation
  (return (+ (Transformation|GetActorLocation Actor) (* (* (Transformation|GetVelocity Actor) "1.000000,1.000000,0.000000") Time))))