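; Attack system component for the third-person character that handles bow aiming.
; It caches the owning character on BeginPlay, then bow input, gated by HasBow, equips the bow and toggles the aiming flag.
; Aiming switches movement to controller-facing rotation and shows a crosshair widget; release restores movement-facing rotation and removes the crosshair after a short delay.
; A debug key unequips the bow from the hands.
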(event Input|EnhancedActionEvents|EnhancedInputActionIA_BowShoot
  (params (ActionValue :type Boolean) (ElapsedSeconds :type Float%20%28double-precision%29) (TriggeredSeconds :type Float%20%28double-precision%29) (InputAction :type Input%20Action%20Object%20Reference :default "/Game/ThirdPerson/Input/Actions/IA_BowShoot.IA_BowShoot"))
  (bind _character_bp (Variables|Default|GetCharacter%20BP))
  (bind _character_bp_2 (Variables|Default|GetCharacter%20BP))
  (bind _charactermovement (Variables|/Script/Engine.Character|GetCharacterMovement _character_bp))
  (bind _charactermovement_2 (Variables|/Script/Engine.Character|GetCharacterMovement _character_bp_2))
  (:Started
    (if (Variables|Default|GetHasBow)
      (Variables|Default|SetCan%20Attack false)
      (Variables|Default|SetAimingBow true)
      (Default|EquipBowinHands _character_bp_2)
      (Variables|/Script/Engine.CharacterMovementComponent|SetbUseControllerDesiredRotation _charactermovement_2 true)
      (Variables|/Script/Engine.CharacterMovementComponent|SetbOrientRotationToMovement _charactermovement_2 false)
      (bind _returnvalue (UserInterface|CreateWidget "/Game/UI/WB_Bow_Crosshair.WB_Bow_Crosshair_C"))
      (bind _output_get (Variables|Default|SetBow%20Crosshair%20Widget _returnvalue))
      (UserInterface|Viewport|AddtoViewport _output_get 0)))
  (:Completed
    (if (Variables|Default|GetHasBow)
      (Variables|Default|SetCan%20Attack false)
      (Variables|Default|SetAimingBow false)
      (Variables|/Script/Engine.CharacterMovementComponent|SetbUseControllerDesiredRotation _charactermovement false)
      (Variables|/Script/Engine.CharacterMovementComponent|SetbOrientRotationToMovement _charactermovement true)
      (Utilities|FlowControl|Delay 0.2)
      (bind _bow_crosshair_widget (Variables|Default|GetBow%20Crosshair%20Widget)
        (:then
          (Widget|RemovefromParent _bow_crosshair_widget)
          (Variables|Default|SetBow%20Crosshair%20Widget 0))
        (:else)))))

(event EventBeginPlay
  (bind _asbp_third_person_character (Utilities|Casting|CastToBP_ThirdPersonCharacter (Components|GetOwner)))
  (Variables|Default|SetCharacter%20BP _asbp_third_person_character)
  (Variables|Default|SetCharacter%20Mesh (Variables|/Script/Engine.Character|GetMesh _asbp_third_person_character)))

(event Input|KeyboardEvents|DebugKeyQ
  (params (Key :type Key%20Structure :default "None") (ActionValue :type Input%20Action%20Value%20Structure))
  (:Pressed
    (if (Variables|Default|GetHasBow)
      (Default|UnequipBowinHands (Variables|Default|GetCharacter%20BP)))))