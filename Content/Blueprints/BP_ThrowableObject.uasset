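; Throwable object that makes a noise the first time its Model component registers a hit.
; The hit event passes through a DoOnce with no reset, so later impacts are ignored.
; That first hit reports an AI noise event at the actor's location, with itself as instigator, and plays a drop sound there.
; Several unconnected noise-report nodes remain in the graph and never run.
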(event OnComponentHit(Model)
  (params (HitComponent :type Primitive%20Component%20Object%20Reference) (OtherActor :type Actor%20Object%20Reference) (OtherComp :type Primitive%20Component%20Object%20Reference) (NormalImpulse :type Vector :default "0, 0, 0") (Hit :type Hit%20Result%20Structure%20%28by%20ref%29))
  (bind _returnvalue (Transformation|GetActorLocation))
  (Utilities|FlowControl|DoOnce false
    (:Completed
      (Class|AISenseHearing|ReportNoiseEvent _returnvalue 1.0 self 0.0 "None")
      (Audio|PlaySoundatLocation "/Engine/VREditor/Sounds/UI/Drop_Item_From_ContentBrowser.Drop_Item_From_ContentBrowser" _returnvalue "0, 0, 0" 1.0 1.0 0.0 "/Game/Audio/SA_Character.SA_Character" 0 0 0))))

(event EventBeginPlay)

(event Collision|EventActorBeginOverlap
  (params (OtherActor :type Actor%20Object%20Reference)))

(event EventTick
  (params (DeltaSeconds :type Float%20%28single-precision%29)))

(fn ConstructionScript)